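; In-game game mode for ByteWars that spawns destruction effects and hands out a shared session ID.
; Ship and missile events spawn explosion actors tinted by team or missile colour, with an extra pulse on the pawn's camera background or a hit star's planet object.
; BeginPlay generates a GUID session ID, which PostLogin passes to the two Odin test components on each joining controller for replication.
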(event `self.OnShipDestroyedFX`
  (params (SourcePlayerController :type "PlayerController Object Reference") (ShipTransform :type "Transform Structure") (ShipPlayerState :type "AccelByteWarsPlayerState Object Reference"))
  ;[0 0 0] FX Event: ship destroyed
  (`|ExecutionSequence`
    (:`then_0`
      ;;[0 0 0] Spawn ship explosion FX
      (bind _returnvalue (`|SpawnActorFromClass` "/Game/ByteWars/Blueprints/Ships/B_ShipExplosion.B_ShipExplosion_C" ShipTransform "Undefined" "OverrideRootScale" SourcePlayerController null))
      (`NiagaraComponent.SetVariableLinearColor` (`AccelByteWarsFxActor.ParticleSystem` _returnvalue) "ShipColour" (`AccelByteWarsPlayerState.TeamColor` ShipPlayerState)))
    (:`then_1`
      ;;[0 0 0] Pulse camera
      (bind _asabpawn (cast `/Game/ByteWars/Blueprints/Player/ABPawn` (`PlayerState.GetPawn` ShipPlayerState)))
      (`AccelByteWarsPlayerPawn.PulseCameraBackground` _asabpawn))))

(event `self.OnMissileDestroyed`
  (params (Location :type "Vector Structure") (HitObject :type "AccelByteWarsGameplayObjectComponent Object Reference") (MissileColour :type "LinearColor Structure") (MissileOwner :type "Actor Object Reference"))
  ;[0 0 0] FX Event: missile destroyed
  (`|ExecutionSequence`
    (:`then_0`
      (bind _returnvalue (`|SpawnActorFromClass` "/Game/ByteWars/Blueprints/Missiles/B_MissileExplosion.B_MissileExplosion_C" (`KismetMathLibrary.MakeTransform` Location) "Undefined" "OverrideRootScale" MissileOwner null))
      (`NiagaraComponent.SetVariableLinearColor` (`AccelByteWarsFxActor.ParticleSystem` _returnvalue) "MissileColour" MissileColour))
    (:`then_1`
      (if (`|EnumEquality` (`AccelByteWarsGameplayObjectComponent.ObjectType` HitObject) "STAR")
        (bind _asb_planet_object (cast `/Game/ByteWars/Blueprints/Planets/B_PlanetObject` (`ActorComponent.GetOwner` HitObject)))
        (`/Game/ByteWars/Blueprints/Planets/B_PlanetObject.PulsePlanet_Event` _asb_planet_object)))))

(event `OnMissileExpired_Event`
  (params (Location :type "Vector Structure") (Color :type "LinearColor Structure") (Owner :type "Actor Object Reference"))
  ;[0 0 0] FX event: missile expired
  (`|SpawnActorFromClass` "/Game/ByteWars/Blueprints/Missiles/B_MissileExpiredExplosion.B_MissileExpiredExplosion_C" (`KismetMathLibrary.MakeTransform` Location) "Undefined" "OverrideRootScale" Owner Color null))

(event `self.ReceiveBeginPlay`
  (`parent.ReceiveBeginPlay`)
  (set `self.SessionId` (`KismetGuidLibrary.Conv_GuidToString` (`KismetGuidLibrary.NewGuid`)))
  (`KismetSystemLibrary.PrintText` (`|FormatText` "Generated Session Id: {sessionId}" (`self.SessionId`))))

(event `self.K2_PostLogin`
  (params (NewPlayer :type "PlayerController Object Reference"))
  (`/Engine/EditorBlueprintResources/StandardMacros.IsValid` NewPlayer
    (:`Is Valid`
      (`|ExecutionSequence`
        (:`then_0`
          (`/Game/Odin/OdinPVCTestComponent_Controller.ReplicateSessionId` (`self.GetComponentByClass` NewPlayer "/Game/Odin/OdinPVCTestComponent_Controller.OdinPVCTestComponent_Controller_C") (`self.SessionId`)))
        (:`then_1`
          (`/Game/Odin/OdinSimpleTestComponent.ReplicateSessionId` (`self.GetComponentByClass` NewPlayer "/Game/Odin/OdinSimpleTestComponent.OdinSimpleTestComponent_C") (`self.SessionId`)))))))

(fn `UserConstructionScript`)