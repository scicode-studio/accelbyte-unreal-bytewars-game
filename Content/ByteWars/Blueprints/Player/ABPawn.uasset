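; Player ship pawn for ByteWars that handles presentation events for HUD feedback and effects.
; Label and power bar events count down timers to toggle their B_HUD widgets; the label also follows the ship's projected screen position, only on listen server and client.
; Other events pulse the B_InGameCamera background, except on dedicated servers, and spawn B_FireMissile at a supplied transform.
; The graph only defines these events; their callers are outside it.
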(event `self.UpdateShipLabelUI`
  (params (DeltaTime :type "Float (single-precision)"))
  (bind _showshiplabeluitimer (`self.ShowShipLabelUITimer`))
  (bind _returnvalue (> _showshiplabeluitimer 0.0))
  ;[0 0 0] Update Ship Label UI
  (`AccelByteWarsBlueprintFunctionLibrary.GetNetMode` null
    (:`ListenServer`
      _)
    (:`Client`
      _))
  (bind _asplayer_controller (cast `PlayerController` (`self.GetController`)))
  (bind _asb_hud (cast `/Game/ByteWars/UI/HUD/B_HUD` (`PlayerController.GetHUD` _asplayer_controller)))
  (bind _shiplabelui (`/Game/ByteWars/UI/HUD/B_HUD.ShipLabelUI` _asb_hud))
  (`/Engine/EditorBlueprintResources/StandardMacros.IsValid` _shiplabelui
    (:`Is Valid`
      (set `self.ShowShipLabelUITimer` (- _showshiplabeluitimer DeltaTime))
      (`/Game/ByteWars/UI/HUD/W_HUD_ShipLabel.UpdateVisibility` _shiplabelui _returnvalue)
      (if _returnvalue
        (`/Game/ByteWars/UI/HUD/W_HUD_ShipLabel.UpdatePosition` _shiplabelui (`GameplayStatics.ProjectWorldToScreen` _asplayer_controller (`self.K2_GetActorLocation`)))))))

(event `self.UpdatePowerBarUI`
  (params (DeltaTime :type "Float (single-precision)"))
  (bind _showpowerleveluitimer (`self.ShowPowerLevelUITimer`))
  ;[0 0 0] Update PowerBar UI
  (bind _asplayer_controller (cast `PlayerController` (`self.GetController`)))
  (bind _asb_hud (cast `/Game/ByteWars/UI/HUD/B_HUD` (`PlayerController.GetHUD` _asplayer_controller)))
  (bind _powerbarui (`/Game/ByteWars/UI/HUD/B_HUD.PowerBarUI` _asb_hud))
  (`/Engine/EditorBlueprintResources/StandardMacros.IsValid` _powerbarui
    (:`Is Valid`
      (if (> _showpowerleveluitimer 0.0)
        (set `self.ShowPowerLevelUITimer` (`KismetMathLibrary.FClamp` (- _showpowerleveluitimer DeltaTime)))
        (`/Game/ByteWars/UI/HUD/W_HUD_ShipPowerBar.Update UI Visibility` _powerbarui true)
        (else
          (`/Game/ByteWars/UI/HUD/W_HUD_ShipPowerBar.Update UI Visibility` _powerbarui false))))))

(event `self.PulseCameraBackground`
  ;[0 0 0] Pulse Camera background
  (if (not (`KismetSystemLibrary.IsDedicatedServer`))
    (bind _returnvalue (`GameplayStatics.GetActorOfClass` "/Game/ByteWars/Blueprints/Cameras/B_InGameCamera.B_InGameCamera_C"))
    (`AccelByteWarsInGameCameraActor.PulseBackground` _returnvalue)))

(event `self.FireMissileFx`
  (params (SpawnTransform :type "Transform Structure"))
  ;[0 0 0] Fire missile fx
  (`|SpawnActorFromClass` "/Game/ByteWars/Blueprints/Ships/B_FireMissile.B_FireMissile_C" SpawnTransform "Undefined" "OverrideRootScale" self self))

(fn `UserConstructionScript`)