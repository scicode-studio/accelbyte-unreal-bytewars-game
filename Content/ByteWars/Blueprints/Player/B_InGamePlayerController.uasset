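; In-game player controller for ByteWars that turns Enhanced Input actions into commands on the controlled ABPawn ship.
; On local BeginPlay, after a short delay, it adds input mappings and switches view to the top-down B_InGameCamera.
; Power, firing and rotation go through Server-prefixed pawn calls, with rotation handlers checking the opposite input to resume that direction.
; The game instance supplies the power-up selection and opens the SDK config menu.
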(event `EnhancedInput|/Game/ByteWars/Blueprints/Input/InputActions/IA_AdjustPower`
  (params (ActionValue :type "Float (double-precision)") (ElapsedSeconds :type "Float (double-precision)") (TriggeredSeconds :type "Float (double-precision)") (InputAction :type "InputAction Object Reference" :default "/Game/ByteWars/Blueprints/Input/InputActions/IA_AdjustPower.IA_AdjustPower"))
  (bind _returnvalue (`self.K2_GetPawn`))
  (bind _returnvalue_2 (`self.K2_GetActorLocation` _returnvalue))
  ;[0 0 0] Adjust Fire Power input listener
  (:`Triggered`
    ;;[0 0 0] Show power level UI
    (bind _asabpawn (cast `/Game/ByteWars/Blueprints/Player/ABPawn` _returnvalue))
    (`AccelByteWarsPlayerPawn.OnPlayerInputThisFrame` _asabpawn))
  (:`Started`
    (`/Engine/EditorBlueprintResources/StandardMacros.IsValid` _returnvalue :!label _label
      (:`Is Valid`
        (bind _asabpawn_2 (cast `/Game/ByteWars/Blueprints/Player/ABPawn` _returnvalue))
        (`/Engine/EditorBlueprintResources/StandardMacros.CompareFloat` ActionValue
          (:`>`
            (`AccelByteWarsPlayerPawn.Server_AdjustFirePower` _asabpawn_2 _returnvalue_2 1))
          (:`==`
            (`AccelByteWarsPlayerPawn.Server_AdjustFirePower` _asabpawn_2 _returnvalue_2 0))
          (:`<`
            (`AccelByteWarsPlayerPawn.Server_AdjustFirePower` _asabpawn_2 _returnvalue_2 2))))))
  (:`Completed`
    (goto _label)))

(event `EnhancedInput|/Game/ByteWars/Blueprints/Input/InputActions/IA_FireMissile`
  (params (ActionValue :type Boolean) (ElapsedSeconds :type "Float (double-precision)") (TriggeredSeconds :type "Float (double-precision)") (InputAction :type "InputAction Object Reference" :default "/Game/ByteWars/Blueprints/Input/InputActions/IA_FireMissile.IA_FireMissile"))
  ;[0 0 0] Fire missile input listener
  (:`Triggered`
    (bind _asabpawn (cast `/Game/ByteWars/Blueprints/Player/ABPawn` (`self.K2_GetPawn`)))
    (`AccelByteWarsPlayerPawn.Server_FireMissile` _asabpawn)))

(event `self.ReceiveBeginPlay`
  (bind _returnvalue (pcsubsystem `EnhancedInputLocalPlayerSubsystem` self))
  ;[0 0 0] BeginPlay sequence
  (`KismetSystemLibrary.Delay` 0.2)
  (if (`self.IsLocalPlayerController`)
    (`EnhancedInputSubsystemInterface.AddMappingContext` _returnvalue "/Game/ByteWars/Blueprints/Input/InputMapping/IM_GlobalDefault.IM_GlobalDefault" 100 (struct))
    (`EnhancedInputSubsystemInterface.AddMappingContext` _returnvalue "/Game/ByteWars/Blueprints/Input/InputMapping/IM_InGameDefault.IM_InGameDefault" 0 (struct))
    (`WidgetBlueprintLibrary.SetInputMode_GameOnly` self)
    (`self.EnableInput` self null)
    ;;[0 0 0] Use top down camera
    (bind _returnvalue_2 (`GameplayStatics.GetActorOfClass` "/Game/ByteWars/Blueprints/Cameras/B_InGameCamera.B_InGameCamera_C"))
    (`self.SetViewTargetWithBlend` _returnvalue_2)))

(event `EnhancedInput|/Game/ByteWars/Blueprints/Input/InputActions/IA_RotateShip_Clockwise`
  (params (ActionValue :type "Float (double-precision)") (ElapsedSeconds :type "Float (double-precision)") (TriggeredSeconds :type "Float (double-precision)") (InputAction :type "InputAction Object Reference" :default "/Game/ByteWars/Blueprints/Input/InputActions/IA_RotateShip_Clockwise.IA_RotateShip_Clockwise"))
  (bind _returnvalue (`self.K2_GetPawn`))
  ;[0 0 0] RotateShip
  (:`Started`
    (`/Engine/EditorBlueprintResources/StandardMacros.IsValid` _returnvalue
      (:`Is Valid`
        (bind _asabpawn (cast `/Game/ByteWars/Blueprints/Player/ABPawn` _returnvalue))
        (`AccelByteWarsPlayerPawn.Server_RotatePawn` _asabpawn 1))))
  (:`Ongoing`
    (`/Engine/EditorBlueprintResources/StandardMacros.IsValid` _returnvalue :!label _label_2
      (:`Is Valid`
        (cast `/Game/ByteWars/Blueprints/Player/ABPawn` _returnvalue)
        (if (< (`|GetInputActionValue`) 0.0)
          (`AccelByteWarsPlayerPawn.Server_RotatePawn` _asabpawn 0)
          (`AccelByteWarsPlayerPawn.Server_RotatePawn` _asabpawn 2)
          (else
            (`AccelByteWarsPlayerPawn.Server_RotatePawn` _asabpawn 0))))))
  (:`Completed`
    (goto _label_2)))

(event `EnhancedInput|/Game/ByteWars/Blueprints/Input/InputActions/IA_RotateShip_CounterClockwise`
  (params (ActionValue :type "Float (double-precision)") (ElapsedSeconds :type "Float (double-precision)") (TriggeredSeconds :type "Float (double-precision)") (InputAction :type "InputAction Object Reference" :default "/Game/ByteWars/Blueprints/Input/InputActions/IA_RotateShip_CounterClockwise.IA_RotateShip_CounterClockwise"))
  (bind _returnvalue (`self.K2_GetPawn`))
  ;[0 0 0] RotateShip
  (:`Started`
    (`/Engine/EditorBlueprintResources/StandardMacros.IsValid` _returnvalue
      (:`Is Valid`
        (bind _asabpawn (cast `/Game/ByteWars/Blueprints/Player/ABPawn` _returnvalue))
        (`AccelByteWarsPlayerPawn.Server_RotatePawn` _asabpawn 2))))
  (:`Ongoing`
    (`/Engine/EditorBlueprintResources/StandardMacros.IsValid` _returnvalue :!label _label_3
      (:`Is Valid`
        (bind _asabpawn_2 (cast `/Game/ByteWars/Blueprints/Player/ABPawn` _returnvalue))
        (if (> (`|GetInputActionValue`) 0.0)
          (`AccelByteWarsPlayerPawn.Server_RotatePawn` _asabpawn_2 0)
          (`AccelByteWarsPlayerPawn.Server_RotatePawn` _asabpawn_2 1)
          (else
            (`AccelByteWarsPlayerPawn.Server_RotatePawn` _asabpawn_2 0))))))
  (:`Completed`
    (goto _label_3)))

(event `EnhancedInput|/Game/ByteWars/Blueprints/Input/InputActions/IA_SdkConfig`
  (params (ActionValue :type Boolean) (ElapsedSeconds :type "Float (double-precision)") (TriggeredSeconds :type "Float (double-precision)") (InputAction :type "InputAction Object Reference" :default "/Game/ByteWars/Blueprints/Input/InputActions/IA_SdkConfig.IA_SdkConfig"))
  ;[0 0 0] Open SDK Config
  (:`Triggered`
    (bind _asaccel_byte_wars_game_instance (cast `AccelByteWarsGameInstance` (`GameplayStatics.GetGameInstance`)))
    (`AccelByteWarsGameInstance.OpenSDKConfigMenu` _asaccel_byte_wars_game_instance)))

(event `EnhancedInput|/Game/ByteWars/Blueprints/Input/InputActions/IA_UsePowerUp`
  (params (ActionValue :type Boolean) (ElapsedSeconds :type "Float (double-precision)") (TriggeredSeconds :type "Float (double-precision)") (InputAction :type "InputAction Object Reference" :default "/Game/ByteWars/Blueprints/Input/InputActions/IA_UsePowerUp.IA_UsePowerUp"))
  (bind _returnvalue (`self.K2_GetPawn`))
  ;[0 0 0] Activate Power Up
  (:`Triggered`
    (`/Engine/EditorBlueprintResources/StandardMacros.IsValid` _returnvalue
      (:`Is Valid`
        (bind _asabpawn (cast `/Game/ByteWars/Blueprints/Player/ABPawn` _returnvalue))
        (`/Engine/EditorBlueprintResources/StandardMacros.IsValid` _asabpawn
          (:`Is Valid`
            (bind _asaccel_byte_wars_game_instance (cast `AccelByteWarsGameInstance` (`GameplayStatics.GetGameInstance`)))
            (`/Engine/EditorBlueprintResources/StandardMacros.IsValid` _asaccel_byte_wars_game_instance
              (:`Is Valid`
                (bind _returnvalue_2 (`AccelByteWarsGameInstance.GetShipPowerUp` _asaccel_byte_wars_game_instance))
                (`AccelByteWarsPlayerPawn.ValidateActivatePowerUp` _asabpawn (cast `EPowerUpSelection` (`KismetMathLibrary.Conv_IntToByte` _returnvalue_2)))))))))))

(fn `UserConstructionScript`)