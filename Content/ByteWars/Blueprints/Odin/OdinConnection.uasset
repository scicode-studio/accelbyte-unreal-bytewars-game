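; Player controller component that connects the local player to an Odin voice chat room.
; On BeginPlay it generates a room token, builds a room with audio processing settings, binds media events and joins, then publishes microphone capture.
; Added media is stored by peer ID and played through an Odin synth component on that peer's pawn, if already registered in PeerToPawn.
; Removed media clears the entry and destroys that synth.
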(event `self.ReceiveBeginPlay`
  (bind _asplayer_controller (cast `PlayerController` (`self.GetOwner`)))
  (if (`Controller.IsLocalPlayerController` _asplayer_controller)
    (`self.Join Odin Room`)))

(event `Join Odin Room`
  (`|ExecutionSequence`
    (:`then_0`
      ;[1 1 1] Setup Odin
      ;;[1 1 1] Generate Room Token
      (bind _returnvalue (`OdinTokenGenerator.GenerateRoomToken` (`OdinTokenGenerator.ConstructTokenGenerator` (`self.Access Key`)) (`self.Room Name`) "Default" "Default"))
      (set `self.RoomToken` _returnvalue)
      ;;[1 1 1] Construct Room Handle with applied settings
      (set `self.RoomHandle` (`OdinRoom.ConstructRoom` (make `OdinApmSettings` true 0.6 0.5 true -30.0 -40.0 true true true "OdinNS_Moderate" true))))
    (:`then_1`
      ;[1 1 1] On Media Added
      (add `OdinRoom.onMediaAdded` (`self.RoomHandle`) (delegate `OnMediaAdded`)))
    (:`then_2`
      ;[1 1 1] On Media Removed
      (add `OdinRoom.onMediaRemoved` (`self.RoomHandle`) (delegate `OnMediaRemoved`)))
    (:`then_3`
      ;[1 1 1] Join Odin Room
      (`OdinRoomJoin.JoinRoom` :`room` (`self.RoomHandle`) :`url` (`self.ServerUrl`) :`token` (`self.RoomToken`) :`onSuccess` (delegate `OnJoinRoomSuccess`)))))

(event `OnMediaAdded`
  (params (peerId :type Integer64) (media :type "OdinPlaybackMedia Object Reference") (properties :type "OdinJsonObject Object Reference") (room :type "OdinRoom Object Reference"))
  (bind (_value _returnvalue) (`BlueprintMapLibrary.Map_Find` (`self.PeerToPawn`) peerId))
  ;[1 1 1] On Media Added
  (`BlueprintMapLibrary.Map_Add` (`self.PeerToMedia`) peerId media)
  ;;[1 1 1] If the peer id has been replicated before the media added event, create odin synth on registered remote character
  (if _returnvalue
    (bind _returnvalue_2 (`|AddComponentByClass` :`self` _value :`Class` "/Script/Odin.OdinSynthComponent"))
    (`OdinSynthComponent.Odin_AssignSynthToMedia` _returnvalue_2 media)
    (`self.Activate` _returnvalue_2 false)))

(event `OnMediaRemoved`
  (params (peerId :type Integer64) (media :type "OdinPlaybackMedia Object Reference") (room :type "OdinRoom Object Reference"))
  (bind (_value _returnvalue) (`BlueprintMapLibrary.Map_Find` (`self.PeerToPawn`) peerId))
  (bind _returnvalue_2 (`Actor.GetComponentByClass` _value "/Script/Odin.OdinSynthComponent"))
  ;[1 1 1] On Media Removed
  ;;[1 1 1] Destroy Odin Synth Component which has been playing back audio from the removed media
  (`BlueprintMapLibrary.Map_Remove` (`self.PeerToMedia`) peerId)
  (if _returnvalue
    (`/Engine/EditorBlueprintResources/StandardMacros.IsValid` _returnvalue_2
      (:`Is Valid`
        (`self.K2_DestroyComponent` _returnvalue_2)))))

(event `OnJoinRoomSuccess`
  (params (roomId :type String) (roomUserData :type "Array of Byte (by ref)") (customer :type String) (ownPeerId :type Integer64) (ownUserId :type String))
  ;[1 1 1] Join Odin Room
  ;;[1 1 1] Setup Audio Capture and connect to Odin Room
  (bind _returnvalue (`OdinFunctionLibrary.CreateOdinAudioCapture`))
  (`AudioCapture.StartCapturingAudio` _returnvalue)
  (`OdinRoomAddMedia.AddMedia` (`self.RoomHandle`) (`OdinFunctionLibrary.Odin_CreateMedia` _returnvalue)))